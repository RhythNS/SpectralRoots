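; Player character Blueprint that handles health feedback, death and respawn presentation.
; The construction script creates a dynamic mesh material, whose Health parameter follows health changes alongside a debug print.
; Death disables input, clears the Animation Blueprint's Alive flag, then after a delay triggers a HUD fade whose completion callback calls Respawn.
; On respawn, it restores the flag, fades the HUD back and re-enables input.
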(event `self.ReceiveTick`
  (params (DeltaSeconds :type "Float (single-precision)")))

(event `self.OnHealthChanged`
  (params (percentLeft :type "Float (single-precision)"))
  (`MaterialInstanceDynamic.SetScalarParameterValue` (`self.HealthMat`) "Health" percentLeft)
  (`KismetSystemLibrary.PrintString` (`KismetStringLibrary.Concat_StrStr` "Health left: " (`KismetStringLibrary.Conv_DoubleToString` percentLeft)) true true (struct :`G` 0.66 :`B` 1.0 :`A` 1.0) 2.0 "HealthLeft"))

(event `self.OnDied`
  (`self.DisableInput` (`CommonStatics.GetPlayerController`))
  (bind _asab_player (cast `/Game/Characters/Player/AB_Player` (`SkeletalMeshComponent.GetAnimInstance` (`self.Mesh`))))
  (set `/Game/Characters/Player/AB_Player.alive` false _asab_player)
  (`KismetSystemLibrary.Delay` 2.0)
  (`SpectralRootsHUD.FadeTo` (`CommonStatics.GetHUD`) (delegate `On Fade In Out Finished`) "FadeIn"))

(event `On Fade In Out Finished`
  (`self.Respawn`))

(event `self.OnRespawned`
  (bind _asab_player (cast `/Game/Characters/Player/AB_Player` (`SkeletalMeshComponent.GetAnimInstance` (`self.Mesh`))))
  (set `/Game/Characters/Player/AB_Player.alive` true _asab_player)
  (`SpectralRootsHUD.FadeTo` (`CommonStatics.GetHUD`) (delegate `CustomEvent`) "FadeOut")
  (`self.EnableInput` (`CommonStatics.GetPlayerController`)))

(event `CustomEvent`)

(fn `UserConstructionScript`
  (bind _returnvalue (`PrimitiveComponent.CreateDynamicMaterialInstance` (`self.Mesh`) 0 "/Game/Characters/Player/M_CubeTest.M_CubeTest" "None"))
  (set `self.HealthMat` _returnvalue))