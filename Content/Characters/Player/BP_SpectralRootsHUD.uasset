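; Player HUD for Spectral Roots that handles screen fades and the pause menu.
; Fadeto runs camera fades to black, from black or both by behaviour, invoking a callback after the fade-time delay.
; Fade in Out issues both fades at once, as its Sequence does not wait on the Delay.
; Pause and UnPause call the game mode and show or remove a lazily created, reused BP_PauseMenu.
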(event `self.FadeTo`
  (params (onFinished :type "Delegate (by ref)") (behaviour :type "FadeBehaviour Enum" :default "FadeInOut"))
  (bind _fadeinouttime (`self.fadeInOutTime`))
  (bind _playercameramanager (`PlayerController.PlayerCameraManager` (`GameplayStatics.GetPlayerController` 0)))
  (switch `FadeBehaviour` behaviour
    (:`FadeInOut`
      (`|ExecutionSequence`
        (:`then_0`
          (`PlayerCameraManager.StartCameraFade` _playercameramanager 0.0 1.0 _fadeinouttime (struct :`A` 1.0) true true :!label _label))
        (:`then_1`
          (`KismetSystemLibrary.Delay` _fadeinouttime :!label _label_2)
          (`self.InvokeFadeCallback` onFinished))
        (:`then_2`
          (`PlayerCameraManager.StartCameraFade` :`self` _playercameramanager :`FromAlpha` 1.0 :`Duration` _fadeinouttime :`bShouldFadeAudio` true :`bHoldWhenFinished` true :!label _label_3))))
    (:`FadeIn`
      (`|ExecutionSequence`
        (:`then_0`
          (goto _label))
        (:`then_1`
          (goto _label_2))))
    (:`FadeOut`
      (`|ExecutionSequence`
        (:`then_0`
          (goto _label_3))
        (:`then_1`
          (goto _label_2))))))

(event `self.Pause`
  (`TreeGameMode.Pause` (`CommonStatics.GetGameMode`))
  (`/Engine/EditorBlueprintResources/StandardMacros.IsValid` (`self.pauseMenu`)
    (:`Is Valid`
      _)
    (:`Is Not Valid`
      (bind _returnvalue (`|GenericCreateObject` self "/Game/UI/Tree/BP_PauseMenu.BP_PauseMenu_C"))
      (bind _output_get (set `self.pauseMenu` _returnvalue))))
  (`UserWidget.AddToViewport` _output_get 0))

(event `self.UnPause`
  (`TreeGameMode.UnPause` (`CommonStatics.GetGameMode`))
  (`Widget.RemoveFromParent` (`self.pauseMenu`)))

(fn `UserConstructionScript`)